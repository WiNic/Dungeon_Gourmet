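; Music player actor that switches between background and fight music according to how many enemies are attacking.
; BeginPlay creates both 2D audio components, playing the background track and keeping the fight track stopped.
; AddEnemyMusic and RemoveEnemyMusic update a zero-clamped attacker count, then call PlayMusic.
; PlayMusic uses paired DoOnce gates that reset each other to cross-fade once per combat state change, respawning either component if it is invalid.
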(event EventBeginPlay
  (bind _returnvalue (Audio|SpawnSound2D "/Game/Audio/Music/M_BG.M_BG" 1.0 1.0 0.0 0 false false))
  (Variables|Default|Setbackground%20music _returnvalue)
  (bind _returnvalue_2 (Audio|SpawnSound2D "/Game/Audio/Music/M_Fight.M_Fight" 0.0 1.0 0.0 0 false false))
  (bind _output_get (Variables|Default|Setfight%20music _returnvalue_2))
  (Audio|Components|Audio|Stop _output_get)
  (Audio|Components|Audio|SetVolumeMultiplier (Variables|Default|Getfight%20music) 1.0 :!class /Script/Engine.AudioComponent))

(fn ConstructionScript)

(fn PlayMusic
  (if (> (Variables|Default|GetenemiesAttacking) 0)
    (Utilities|FlowControl|Sequence
      (:then_0
        (goto _label_2 Reset))
      (:then_1
        (Utilities|FlowControl|DoOnce false :!label _label
          (:Completed
            ;[1 1 1] Fight Music
            (bind _fight_music (Variables|Default|Getfight%20music)
              (:then
                (if (not (Audio|Components|Audio|IsPlaying _fight_music))
                  (Audio|Components|Audio|FadeIn (stale _output_get) 1.0 1.0 0.0 "Linear" :!class /Script/Engine.AudioComponent)
                  (bind _background_music (Variables|Default|Getbackground%20music)
                    (:then
                      ;[1 1 1] Background Music
                      (Audio|Components|Audio|FadeOut _background_music 1.0 0.0 "Linear" :!class /Script/Engine.AudioComponent))
                    (:else))))
              (:else
                (bind _returnvalue (Audio|SpawnSound2D "/Game/Audio/Music/M_Fight.M_Fight" 1.0 1.0 0.0 0 false false))
                (bind _output_get (Variables|Default|Setfight%20music _returnvalue))))))))
    (else
      (Utilities|FlowControl|Sequence
        (:then_0
          (goto _label Reset))
        (:then_1
          (Utilities|FlowControl|DoOnce false :!label _label_2
            (:Completed
              (bind _background_music_2 (Variables|Default|Getbackground%20music)
                (:then
                  (if (not (Audio|Components|Audio|IsPlaying _background_music_2))
                    (Audio|Components|Audio|FadeIn (stale _output_get_2) 1.0 1.0 0.0 "Linear" :!class /Script/Engine.AudioComponent)
                    (bind _fight_music_2 (Variables|Default|Getfight%20music)
                      (:then
                        (Audio|Components|Audio|FadeOut _fight_music_2 1.0 0.0 "Linear" :!class /Script/Engine.AudioComponent))
                      (:else))))
                (:else
                  (bind _returnvalue_2 (Audio|SpawnSound2D "/Game/Audio/Music/M_BG.M_BG" 1.0 1.0 0.0 0 false false))
                  (bind _output_get_2 (Variables|Default|Setbackground%20music _returnvalue_2)))))))))))

(fn AddEnemyMusic
  (Variables|Default|SetenemiesAttacking (+ (Math|Integer|Max(Integer) (Variables|Default|GetenemiesAttacking)) 1))
  (CallFunction|PlayMusic))

(fn RemoveEnemyMusic
  (Variables|Default|SetenemiesAttacking (Math|Integer|Max(Integer) (- (Variables|Default|GetenemiesAttacking) 1)))
  (CallFunction|PlayMusic))