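; Enemy spawner actor that queues enemy classes and spawns them near itself while the world's EnemyAI count is under MaxEnemys.
; AddEnemyToQueue appends valid classes, then tries an immediate spawn unless that class overlaps NoSpawnZone.
; A looping timer, its interval randomized once at BeginPlay, also retries without that zone check.
; SpawnEnemy takes the oldest entry, spawning it with random offset and yaw.
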(event Custom|TryToSpawn
  (CallFunction|SpawnEnemy))

(event EventBeginPlay
  (Utilities|Time|SetTimerbyEvent (delegate Custom|TryToSpawn) (Math|Random|RandomFloatinRange 0.5 3.0) true))

(fn ConstructionScript)

(fn SpawnEnemy
  ;[1 1 1] check performance
  (bind _outactors (Actor|GetAllActorsOfClass "/Game/Characters/Enemy/EnemyAI.EnemyAI_C"))
  (if (and (< (Utilities|Array|Length _outactors) (Variables|Default|GetmaxEnemys)) (Utilities|Array|IsValidIndex (Variables|Default|GetEnemyQueue)))
    (Game|SpawnActorfromClass (Utilities|Array|Get(acopy) (Variables|Default|GetEnemyQueue)) (Math|Transform|MakeTransform (+ (Transformation|GetActorLocation) (Math|Vector|MakeVector (Math|Random|RandomFloatinRange 0.0 5e+01) (Math|Random|RandomFloatinRange 0.0 5e+01) 0.0)) (Math|Rotator|MakeRotator 0.0 0.0 (Math|Random|RandomFloatinRange 0.0 1.8e+02))) "Undefined" 0 0 0)
    (Utilities|Array|RemoveIndex (Variables|Default|GetEnemyQueue))
    (return true)
    (else
      (return false))))

(fn AddEnemytoQueue
  (params (EnemyClass :type Enemy%20AI%20Class%20Reference%20%28by%20ref%29))
  (if (Utilities|IsValidClass EnemyClass)
    (Utilities|Array|Add (Variables|Default|GetEnemyQueue) EnemyClass)
    (if (not (Utilities|Array|IsValidIndex (Collision|GetOverlappingActors (Variables|Default|GetNoSpawnZone) EnemyClass :!class /Script/Engine.PrimitiveComponent)))
      (CallFunction|SpawnEnemy))))