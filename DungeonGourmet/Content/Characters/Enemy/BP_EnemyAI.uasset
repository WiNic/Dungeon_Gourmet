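; Enemy AI character that chases a seen player and performs melee attacks while alive.
; Pawn sensing starts AIMoveTo and a looping timed yaw update toward the player; arrival fires a DoOnce-gated montage that halts movement.
; A montage notify runs a forward sphere trace dealing randomized damage, then completion restores speed and unlocks the next attack.
; Untested damage handling sets hit points to damage minus current points and updates the alive flag.
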(event OnSeePawn(PawnSensing)
  (params (Pawn :type Pawn%20Object%20Reference))
  (bind _charactermovement (Variables|Character|GetCharacterMovement))
  ;[1 1 1] AI Movement
  (bind _asbp_third_person_character (Utilities|Casting|CastToBP_ThirdPersonCharacter Pawn))
  (bind _output_get (Variables|Default|SetPlayer _asbp_third_person_character))
  (if (Variables|Default|GetAlive)
    (AI|AIMoveTo self "0, 0, 0" _output_get (Variables|Default|GetAttackRadius) true
      (:then
        (CallFunction|LookatPlayer))
      (:OnSuccess
        ;[1 1 1] Attack when in range
        (Utilities|FlowControl|DoOnce false
          (:Completed
            (bind _notifyname (Animation|Montage|PlayMontage (Variables|Character|GetMesh) (Variables|Default|GetAttackMontage))
              (:then
                (Components|Movement|StopMovementImmediately _charactermovement)
                (Variables|/Script/Engine.CharacterMovementComponent|SetMaxWalkSpeed _charactermovement 0.0))
              (:OnCompleted
                (Utilities|FlowControl|Delay 0.2)
                (CallFunction|UnlockAttack)
                (Variables|/Script/Engine.CharacterMovementComponent|SetMaxWalkSpeed _charactermovement (Variables|Default|GetMaxMoveSpeed)))
              (:OnNotifyBegin
                (switch name _notifyname
                  (:AttackTrace
                    (CallFunction|AttackTrace)))))))))
    (else
      (CallFunction|GetAlive))))

(event Custom|unlockAttack
  (bind _charactermovement (Variables|Character|GetCharacterMovement))
  ;[1 1 1] Attack when in range
  (Utilities|FlowControl|DoOnce false) ; enters at Reset
)

(event Custom|LookAtPlayer
  ;[1 1 1] Rotate to look at Player. Makes a smooth turn animations
  (bind _player (Variables|Default|GetPlayer)
    (:then
      (Transformation|SetActorRotation (Math|Rotator|MakeRotator 0.0 0.0 (.yaw (Math|Rotator|FindLookatRotation (Transformation|GetActorLocation) (Transformation|GetActorLocation _player)))))
      (Utilities|FlowControl|Delay 0.01)
      (CallFunction|LookatPlayer))
    (:else)))

(event EventBeginPlay)

(event Collision|EventActorBeginOverlap
  (params (OtherActor :type Actor%20Object%20Reference)))

(event EventTick
  (params (DeltaSeconds :type Float%20%28single-precision%29)))

(event Game|Damage|EventAnyDamage
  (params (Damage :type Float%20%28single-precision%29) (DamageType :type Damage%20Type%20Object%20Reference) (InstigatedBy :type Controller%20Object%20Reference) (DamageCauser :type Actor%20Object%20Reference))
  ;[1 1 1] Not Tested
  (Variables|Default|SetCurrentHitPoints (- Damage (Variables|Default|GetCurrentHitPoints)))
  (Variables|Default|SetAlive (> (Variables|Default|GetCurrentHitPoints) 0.0)))

(fn ConstructionScript)

(fn AttackTrace
  (bind _returnvalue (Transformation|GetActorLocation))
  (bind _attackdmg (Variables|Default|GetAttackDmg))
  (bind _attackdmgvariance (Variables|Default|GetAttackDmgVariance))
  (bind (_outhit _returnvalue_2) (Collision|SphereTraceByChannel _returnvalue (+ _returnvalue (* (Transformation|GetActorForwardVector) (Variables|Default|GetAttackRange))) (Variables|Default|GetAttackRadius) "TraceTypeQuery1" false 0 "ForDuration"))
  (if _returnvalue_2
    (Game|Damage|ApplyDamage (.HitActor (Collision|BreakHitResult _outhit)) (Math|Conversions|ToFloat(Integer) (Class|KismetMathLibrary|Round64 (Math|Random|RandomFloatinRange (- _attackdmg _attackdmgvariance) (+ _attackdmg _attackdmgvariance)))) 0 0)))

(fn GetAlive
  (return (Variables|Default|GetAlive)))