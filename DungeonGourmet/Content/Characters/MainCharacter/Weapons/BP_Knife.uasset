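; BP_Knife is a knife projectile in the main character's weapons, moved by a ProjectileMovement component.
; Construction applies Speed as both its initial and max speed.
; On BeginPlay with a valid Emitter, it aims straight at the Target if valid, otherwise rotates its current velocity by VelocityRotation.
; Both paths add the emitter's velocity, and the aim is set only once, with no homing logic in the graph.
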(event Custom|RotateToTarget
  (bind _emitter (Variables|Default|GetEmitter))
  ;[1 1 1] Rotate from emitter to target actor +  add emitter velocity
  (Variables|/Script/Engine.MovementComponent|SetVelocity (Variables|Default|GetProjectileMovement) (+ (Transformation|GetVelocity _emitter) (* (Math|Vector|GetUnitDirection(Vector) (Transformation|GetActorLocation _emitter) (Transformation|GetActorLocation (Variables|Default|GetTarget))) (Variables|ProjectileSettings|GetSpeed)))))

(event EventBeginPlay
  (Variables|Default|GetEmitter
    (:then
      (Variables|Default|GetTarget
        (:then
          (CallFunction|RotatetoTarget))
        (:else
          ;[1 1 1] Rotate velocity given a local rotator +  add emitter velocity
          (Variables|/Script/Engine.MovementComponent|SetVelocity (Variables|Default|GetProjectileMovement) (+ (Transformation|GetVelocity (Variables|Default|GetEmitter)) (Math|Vector|RotateVector (Transformation|GetVelocity) (Variables|Default|GetVelocityRotation)))))))
    (:else)))

(event Collision|EventActorBeginOverlap
  (params (OtherActor :type Actor%20Object%20Reference)))

(event EventTick
  (params (DeltaSeconds :type Float%20%28single-precision%29)))

(fn ConstructionScript
  (bind _projectilemovement (Variables|Default|GetProjectileMovement))
  (Variables|/Script/Engine.ProjectileMovementComponent|SetInitialSpeed _projectilemovement (Variables|ProjectileSettings|GetSpeed))
  (Variables|/Script/Engine.ProjectileMovementComponent|SetMaxSpeed _projectilemovement (Variables|ProjectileSettings|GetSpeed)))